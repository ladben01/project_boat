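; BP_PlayerStart is a player start point that rates itself by its distance from the boats in the level.
; On BeginPlay it runs CalculateSpawnScore, which finds every Boat actor and adds its straight-line distance from this start to SpawnScore.
; The event adds to the existing score without resetting it, and nothing in this graph reads the result.
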(event Custom|CalculateSpawnScore
  (bind _outactors (Actor|GetAllActorsOfClass "/Script/ProjectBoat.Boat"))
  (for _array_element _outactors
    (Variables|Default|SetSpawnScore (+ (Math|Vector|VectorLength (- (Transformation|GetActorLocation _array_element) (Transformation|GetActorLocation))) (Variables|Default|GetSpawnScore)))))

(event EventBeginPlay
  (CallFunction|CalculateSpawnScore))

(fn ConstructionScript)