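; Player boat pawn with mouse-orbit camera, ship-type setup, debug toggle and respawn at player start.
; Tick line-traces from the camera and spawns a flare as the live bullet's homing target, using a server RPC on clients.
; Bullet, torpedo and smoke spawn events remain, but their triggering chains are disconnected.
; Optionally registers its front with BP_FluidSim_01 for water forces; a trace-based DoBuoyancy helper is defined but uncalled here.
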(event Custom|Server_ResetPlayer
  (bind _returnvalue (Game|GetGameMode))
  (bind _returnvalue_2 (Pawn|GetController))
  (bind _asproject_boat_game_mode_base (Utilities|Casting|CastToProjectBoatGameModeBase _returnvalue))
  (bind _returnvalue_3 (Class|GameModeBase|FindPlayerStart _asproject_boat_game_mode_base _returnvalue_2))
  (CallFunction|ClientResetPlayer (Transformation|GetActorLocation _returnvalue_3) (Transformation|GetActorRotation _returnvalue_3)))

(event Custom|Client_ResetPlayer
  (params (Location :type Vector) (Rotation :type Rotator))
  (Class|Boat|Die Location Rotation))

(event Custom|Server_SpawnTarget
  (params (Spawn%20Transform%20Location :type Vector))
  (bind _bullet (Variables|Default|GetBullet))
  (bind _projectilemovement (Variables|/Game/ProjectBoat/Characters/BP_TestBullet.BP_TestBullet_C|GetProjectileMovement _bullet))
  (bind _returnvalue (Niagara|SpawnSystematLocation "/Game/Niagara/NE_Flare_System.NE_Flare_System" Spawn%20Transform%20Location))
  (Rendering|SetVisibility _returnvalue false false)
  (Variables|/Script/Engine.ProjectileMovementComponent|SetHomingTargetComponent _projectilemovement _returnvalue)
  (Variables|/Script/Engine.ProjectileMovementComponent|SetbIsHomingProjectile _projectilemovement true))

(event Custom|Server_Smoke
  (CallFunction|MulticastSmoke))

(event Custom|Multicast_Smoke
  (CallFunction|SpawnSmoke))

(event Custom|SpawnSmoke
  (Utilities|IsValid (Variables|Default|GetSmoke)
    (:Is%20Not%20Valid
      (bind _returnvalue (Niagara|SpawnSystematLocation "/Game/Niagara/NE_Smoke_System.NE_Smoke_System" (Transformation|GetActorLocation)))
      (Variables|Default|SetSmoke _returnvalue))))

(event Custom|Server_SpawnTorpedo
  (params (Spawn%20Transform%20Location :type Vector) (Spawn%20Transform%20Rotation :type Rotator))
  (CallFunction|SpawnTorpedo Spawn%20Transform%20Location Spawn%20Transform%20Rotation))

(event Custom|Server_SpawnBullet
  (Utilities|IsValid (Variables|Default|GetBullet)
    (:Is%20Not%20Valid
      (bind _returnvalue (Game|SpawnActorfromClass "/Game/ProjectBoat/Characters/BP_TestBullet.BP_TestBullet_C" (Math|Transform|MakeTransform (+ (Transformation|GetActorLocation) "0, 0,1000.000000") "90.000000, 0, 0" "1,1,1") "Undefined" 0 0))
      (Variables|Default|SetBullet _returnvalue))))

(event Custom|SpawnTorpedo
  (params (Spawn%20Transform%20Location :type Vector) (Spawn%20Transform%20Rotation :type Rotator))
  (Utilities|IsValid (Variables|Default|GetTorpedo)
    (:Is%20Not%20Valid
      (bind _returnvalue (Game|SpawnActorfromClass "/Game/ProjectBoat/Characters/BP_TestTorpedo.BP_TestTorpedo_C" (Math|Transform|MakeTransform Spawn%20Transform%20Location Spawn%20Transform%20Rotation "1,1,1") "Undefined" 0 0))
      (Variables|Default|SetTorpedo _returnvalue)
      (Audio|PlaySoundatLocation "/Game/Sounds/TorpedoLaunch.TorpedoLaunch" Spawn%20Transform%20Location "0, 0, 0" 1.0 1.0 0.0 0 0 0))))

(event EventBeginPlay
  (if (Variables|Default|GetIsFluidSimEnabled)
    (Utilities|FlowControl|Delay 1.0)
    (bind _returnvalue (Actor|GetActorOfClass "/Water/FluidSimulation/Blueprints/BP_FluidSim_01.BP_FluidSim_01_C"))
    (Variables|Default|SetSim _returnvalue)
    (Utilities|Struct|SetmembersinFluidForceDynamic (Variables|Default|GetDynamic%20Fluid%20Force) (Variables|Default|Getfront))
    (Default|RegisterDynamicForce (Variables|Default|GetSim) (Variables|Default|GetDynamic%20Fluid%20Force) (Variables|Default|Getfront) 1.3e+02)))

(event EventOnDeath
  (bind _returnvalue (Game|GetGameMode))
  (bind _returnvalue_2 (Pawn|GetController))
  (bind _asproject_boat_game_mode_base (Utilities|Casting|CastToProjectBoatGameModeBase _returnvalue))
  (bind _returnvalue_3 (Class|GameModeBase|FindPlayerStart _asproject_boat_game_mode_base _returnvalue_2))
  (Networking|SwitchHasAuthority
    (:Authority
      (Class|Boat|Die (Transformation|GetActorLocation _returnvalue_3) (Transformation|GetActorRotation _returnvalue_3)))
    (:Remote
      (CallFunction|ServerResetPlayer))))

(event EventTick
  (params (DeltaSeconds :type Float%20%28single-precision%29))
  (bind _bullet (Variables|Default|GetBullet))
  (bind _camera (Variables|Default|GetCamera))
  (bind _returnvalue (Transformation|GetWorldLocation _camera))
  (bind _returnvalue_2 (Math|Vector|GetForwardVector _camera))
  (bind _projectilemovement (Variables|/Game/ProjectBoat/Characters/BP_TestBullet.BP_TestBullet_C|GetProjectileMovement _bullet))
  (bind _returnvalue_3 (* _returnvalue_2 1.5e+04))
  (bind _returnvalue_4 (+ _returnvalue "0, 0,2500.000000"))
  (bind _returnvalue_5 (+ _returnvalue_4 _returnvalue_3))
  (bind (_x _y) (Math|Vector|BreakVector _returnvalue_5))
  (bind _returnvalue_6 (Math|Vector|MakeVector _x _y 0.0))
  ;[1 1 1] Tick
  ;;[1 1 1] Debug: Log movement speed in km/h
  (if (Pawn|IsLocallyControlled)
    (bind _asproject_boat_player_state (Utilities|Casting|CastToProjectBoatPlayerState (Variables|Default|GetPlayerState))
      (:then
        (bind _returnvalue_7 (Class|ProjectBoatPlayerState|GetDebugMode _asproject_boat_player_state))
        (if _returnvalue_7
          (bind _returnvalue_8 (Physics|GetPhysicsLinearVelocity (Variables|Default|GetBoatMesh) "None"))
          (Development|PrintString (Utilities|String|ToString(Float) (/ (Math|Vector|VectorLength _returnvalue_8) 27.777777)) true false "(R=0.000000,G=0.660000,B=1.000000,A=1.000000)" DeltaSeconds)))
      (:CastFailed
        _))
    (Utilities|IsValid (Variables|Default|GetBullet)
      (:Is%20Valid
        (bind (_outhit _returnvalue_9) (Collision|LineTraceForObjects _returnvalue_4 _returnvalue_5 (Utilities|Array|MakeArray (Utilities|Enum|LiteralenumEObjectTypeQuery "ObjectTypeQuery1")) false 0 "ForOneFrame"))
        (if _returnvalue_9
          (bind _returnvalue_10 (Niagara|SpawnSystematLocation "/Game/Niagara/NE_Flare_System.NE_Flare_System" (.location _outhit)))
          (Networking|SwitchHasAuthority
            (:Authority
              (Variables|/Script/Engine.ProjectileMovementComponent|SetHomingTargetComponent _projectilemovement _returnvalue_10)
              (Variables|/Script/Engine.ProjectileMovementComponent|SetbIsHomingProjectile _projectilemovement true :!label _label))
            (:Remote
              (CallFunction|ServerSpawnTarget (.location _outhit))))
          (else
            (bind _returnvalue_11 (Niagara|SpawnSystematLocation "/Game/Niagara/NE_Flare_System.NE_Flare_System" _returnvalue_6))
            (Networking|SwitchHasAuthority
              (:Authority
                (Variables|/Script/Engine.ProjectileMovementComponent|SetHomingTargetComponent _projectilemovement _returnvalue_11)
                (goto _label))
              (:Remote
                (CallFunction|ServerSpawnTarget _returnvalue_6))))))
      (:Is%20Not%20Valid))))

(event Input|ActionEvents|InputActionToggleDebugMode
  (params (Key :type Key%20Structure :default "None"))
  ;[1 1 1] Handle Debug mode
  (:Pressed
    (bind _asproject_boat_player_state (Utilities|Casting|CastToProjectBoatPlayerState (Variables|Default|GetPlayerState)))
    (Class|ProjectBoatPlayerState|ToggleDebugMode _asproject_boat_player_state)
    (bind _returnvalue (Class|ProjectBoatPlayerState|GetDebugMode _asproject_boat_player_state))
    (bind _outactors (Actor|GetAllActorsOfClass "/Script/ProjectBoat.Boat"))
    (for _array_element _outactors
      (Variables|/Script/ProjectBoat.BoatMovementComponent|SetDebugMode (Variables|/Script/ProjectBoat.Boat|GetMovementComponent _array_element) _returnvalue))))

(event Input|ActionEvents|InputActionRespawnBoat
  (params (Key :type Key%20Structure :default "None"))
  (bind _returnvalue (Game|GetGameMode))
  (bind _returnvalue_2 (Pawn|GetController))
  (bind _asproject_boat_game_mode_base (Utilities|Casting|CastToProjectBoatGameModeBase _returnvalue))
  (bind _returnvalue_3 (Class|GameModeBase|FindPlayerStart _asproject_boat_game_mode_base _returnvalue_2))
  (:Pressed
    (Networking|SwitchHasAuthority
      (:Authority
        (Class|Boat|Die (Transformation|GetActorLocation _returnvalue_3) (Transformation|GetActorRotation _returnvalue_3)))
      (:Remote
        (CallFunction|ServerResetPlayer)))))

(event Input|MouseEvents|MouseX
  (params (AxisValue :type Float%20%28single-precision%29))
  (bind _cameraarm (Variables|Default|GetCameraArm))
  (bind _relativerotation (Variables|/Script/Engine.SceneComponent|GetRelativeRotation _cameraarm))
  ;[1 1 1] Camera movement
  (Transformation|SetRelativeRotation _cameraarm (Math|Rotator|MakeRotator (.roll _relativerotation) (.pitch _relativerotation) (+ (.yaw _relativerotation) AxisValue)) false false))

(event Input|MouseEvents|MouseY
  (params (AxisValue :type Float%20%28single-precision%29))
  (bind _cameraarm (Variables|Default|GetCameraArm))
  (bind _relativerotation (Variables|/Script/Engine.SceneComponent|GetRelativeRotation _cameraarm))
  (bind _returnvalue (+ (.pitch _relativerotation) AxisValue))
  ;[1 1 1] Camera movement
  (if (and (< -7e+01 _returnvalue) (> 1e+01 _returnvalue))
    (Transformation|SetRelativeRotation _cameraarm (Math|Rotator|MakeRotator (.roll _relativerotation) _returnvalue (.yaw _relativerotation)) false false)))

(event Input|MouseEvents|LeftMouseButton
  (params (Key :type Key%20Structure :default "None")))

(event Input|MouseEvents|RightMouseButton
  (params (Key :type Key%20Structure :default "None")))

(event Input|KeyboardEvents|F
  (params (Key :type Key%20Structure :default "None")))

(event Input|KeyboardEvents|H
  (params (Key :type Key%20Structure :default "None")))

(fn ConstructionScript
  (bind _returnvalue (Class|Boat|GetShipType))
  (Class|Boat|SetupShip _returnvalue)
  (Class|ProjectBoatGameInstance|SetShipType (.AsProject%20Boat%20Game%20Instance (Utilities|Casting|CastToProjectBoatGameInstance (Game|GetGameInstance))) _returnvalue)
  (if (Variables|Default|GetIsFluidSimEnabled)
    (bind _returnvalue_2 (Actor|GetActorOfClass "/Water/FluidSimulation/Blueprints/BP_FluidSim_01.BP_FluidSim_01_C"))
    (Variables|Default|SetSim _returnvalue_2)
    (Utilities|Struct|SetmembersinFluidForceDynamic (Variables|Default|GetDynamic%20Fluid%20Force) (Variables|Default|Getfront))
    (Default|RegisterDynamicForce (Variables|Default|GetSim) (Variables|Default|GetDynamic%20Fluid%20Force) (Variables|Default|Getfront) 1.3e+02)))

(fn DoBuoyancy
  (params (Arrow :type Arrow%20Component%20Object%20Reference))
  (bind _returnvalue (Transformation|GetWorldLocation Arrow))
  (bind _returnvalue_2 (Math|Vector|GetUpVector Arrow))
  (bind _returnvalue_3 (Utilities|Enum|LiteralenumEObjectTypeQuery "ObjectTypeQuery1"))
  (bind _returnvalue_4 (* _returnvalue_2 3e+03))
  (bind _array (Utilities|Array|MakeArray _returnvalue_3))
  (bind _returnvalue_5 (+ _returnvalue _returnvalue_4))
  (bind _outhits (Class|KismetSystemLibrary|LineTraceMultiforObjects _returnvalue _returnvalue_5 _array false 0 "ForOneFrame" true))
  (bind (_outhit _returnvalue_6) (Collision|LineTraceForObjects _returnvalue _returnvalue_5 _array false (Utilities|Array|MakeArray self) "None"))
  (if (and _returnvalue_6 (.bSuccess (Utilities|Casting|CastToWaterBody (.hitactor _outhit))))
    (Development|PrintString (Utilities|String|ToString(Float) (.distance (Utilities|Array|Get(acopy) _outhits (Utilities|Array|LastIndex _outhits)))))
    (Class|PrimitiveComponent|AddForceatLocation (Variables|Default|GetBoatMesh) (* "0, 0,10000000.000000" (.distance (Utilities|Array|Get(acopy) _outhits (Utilities|Array|LastIndex _outhits)))) _returnvalue "None")))