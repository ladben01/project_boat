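; BP_TestBullet is a projectile power-up actor that knocks boats around on impact.
; Mesh collision stays off for a short delay after spawn, then switches to query and physics.
; On hit, it applies a constant-falloff radial impulse to a struck Boat's mesh at the hit location.
; It then notifies the owning Boat's PowerUpComponent of its destruction and destroys itself, whatever it hit.
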(event EventBeginPlay
  (bind _projectilemesh (Variables|Default|GetProjectileMesh))
  (Collision|SetCollisionEnabled _projectilemesh "NoCollision")
  (Utilities|FlowControl|Delay 0.6)
  (Collision|SetCollisionEnabled _projectilemesh "QueryAndPhysics"))

(event Collision|EventHit
  (params (MyComp :type Primitive%20Component%20Object%20Reference) (Other :type Actor%20Object%20Reference) (OtherComp :type Primitive%20Component%20Object%20Reference) (bSelfMoved :type Boolean) (HitLocation :type Vector :default "0, 0, 0") (HitNormal :type Vector :default "0, 0, 0") (NormalImpulse :type Vector :default "0, 0, 0") (Hit :type Hit%20Result%20Structure%20%28by%20ref%29))
  (bind _asboat (Utilities|Casting|CastToBoat Other)
    (:then
      (Physics|AddRadialImpulse (Variables|/Script/ProjectBoat.Boat|GetBoatMesh _asboat) HitLocation 3e+03 1e+05 "RIF_Constant" false))
    (:CastFailed
      _))
  (bind _asboat_2 (Utilities|Casting|CastToBoat (Components|GetOwner))
    (:then
      (Class|BoatPowerUpComponent|OnPowerUpActorDestroyed (Variables|/Script/ProjectBoat.Boat|GetPowerUpComponent _asboat_2) self))
    (:CastFailed
      _))
  (Actor|DestroyActor))

(fn ConstructionScript)