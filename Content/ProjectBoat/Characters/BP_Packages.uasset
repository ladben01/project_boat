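; BP_Packages is an actor that builds stacks of packages with an Instanced Static Mesh and randomized per-instance variation.
; With IsRandom on, the construction script fills a centered Width × Length × Height grid, occasionally cutting columns short.
; Each instance gets two random custom data values, presumably for material variation.
; With it off, existing instances get new values at construction and again at BeginPlay, which also prints debug output.
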(event EventBeginPlay
  (bind _returnvalue (Math|Random|RandomFloatinRange -1.0 2.9999))
  (bind _instancedstaticmesh (Variables|Default|GetInstancedStaticMesh))
  (bind _returnvalue_2 (Math|Float|Ceil _returnvalue))
  (bind _returnvalue_3 (Components|InstancedStaticMesh|GetInstanceCount _instancedstaticmesh))
  (bind _returnvalue_4 (Math|Conversions|ToFloat(Integer) _returnvalue_2))
  (Development|PrintString (Utilities|String|ToString(Integer) _returnvalue_3))
  (if (and (not (Variables|Default|GetIsRandom)) (> _returnvalue_3 0))
    (for _index (range 0 (- _returnvalue_3 1))
      (Components|InstancedStaticMesh|SetCustomDataValue _instancedstaticmesh _index 0 _returnvalue_4 false)
      (Development|PrintString (Utilities|String|ToString(Float) _returnvalue_4))
      (Components|InstancedStaticMesh|SetCustomDataValue _instancedstaticmesh _index 1 (Math|Conversions|ToFloat(Integer) (Math|Float|Ceil (Math|Random|RandomFloatinRange -1.0 2.9999))) false))))

(fn ConstructionScript
  (bind _instancedstaticmesh (Variables|Default|GetInstancedStaticMesh))
  (bind _instancedstaticmesh_2 (Variables|Default|GetInstancedStaticMesh))
  (bind _width (Variables|Default|GetWidth))
  (bind _length (Variables|Default|GetLength))
  (bind _meshlength (Variables|Default|GetMeshLength))
  (bind _returnvalue (- _width 1))
  (bind _returnvalue_2 (- _length 1))
  (bind _returnvalue_3 (Components|InstancedStaticMesh|GetInstanceCount _instancedstaticmesh_2))
  (if (Variables|Default|GetIsRandom)
    (if (> (* (Variables|Default|GetWidth) (Variables|Default|GetLength) (Variables|Default|GetHeight)) 0)
      (bind _index (Utilities|FlowControl|ForLoopwithBreak 0 _returnvalue)
        (:LoopBody
          (bind _index_2 (Utilities|FlowControl|ForLoopwithBreak 0 _returnvalue_2)
            (:LoopBody
              (bind _index_3 (Utilities|FlowControl|ForLoopwithBreak 0 (- (Variables|Default|GetHeight) 1) :!label _label)
                (:LoopBody
                  (if (< (Math|Random|RandomIntegerinRange 0 99) 96)
                    (bind _returnvalue_4 (Components|InstancedStaticMesh|AddInstance _instancedstaticmesh (Math|Transform|MakeTransform (+ (Math|Vector|MakeVector (* (* _returnvalue_2 _meshlength) -0.5) (* (* _returnvalue (Variables|Default|GetMeshWidth)) -0.5) (* (Variables|Default|GetMeshHeight) 0.5)) (Math|Vector|MakeVector (* _index_2 _meshlength) (* _index (Variables|Default|GetMeshWidth)) (* _index_3 (Variables|Default|GetMeshHeight)))) "0, 0, 0" "1,1,1")))
                    (Components|InstancedStaticMesh|SetCustomDataValue _instancedstaticmesh _returnvalue_4 0 (Math|Conversions|ToFloat(Integer) (Math|Float|Ceil (Math|Random|RandomFloatinRange -1.0 2.9999))) false)
                    (Components|InstancedStaticMesh|SetCustomDataValue _instancedstaticmesh _returnvalue_4 1 (Math|Conversions|ToFloat(Integer) (Math|Float|Ceil (Math|Random|RandomFloatinRange -1.0 2.9999))) false)
                    (else
                      (goto _label Break))))))))))
    (elif (> _returnvalue_3 0)
      (for _index_4 (range 0 (- _returnvalue_3 1))
        (Components|InstancedStaticMesh|SetCustomDataValue _instancedstaticmesh_2 _index_4 0 (Math|Conversions|ToFloat(Integer) (Math|Float|Ceil (Math|Random|RandomFloatinRange -1.0 2.9999))) false)
        (Components|InstancedStaticMesh|SetCustomDataValue _instancedstaticmesh_2 _index_4 1 (Math|Conversions|ToFloat(Integer) (Math|Float|Ceil (Math|Random|RandomFloatinRange -1.0 2.9999))) false)))))