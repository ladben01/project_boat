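; Container prop actor for the Central Port, built on an instanced static mesh component.
; Its Construction Script loops over every instance and writes independent random whole numbers, effectively 0 to 3, into the first two custom data slots.
; These per-instance values can drive material variation without separate meshes, and are re-rolled whenever construction runs.
; The event graph holds no active logic.
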(event EventBeginPlay)

(event Collision|EventActorBeginOverlap
  (params (OtherActor :type Actor%20Object%20Reference)))

(event EventTick
  (params (DeltaSeconds :type Float%20%28single-precision%29)))

(fn ConstructionScript
  (bind _instancedstaticmesh (Variables|Default|GetInstancedStaticMesh))
  (bind _returnvalue (Components|InstancedStaticMesh|GetInstanceCount _instancedstaticmesh))
  (if (> _returnvalue 0)
    (for _index (range 0 (- _returnvalue 1))
      (Components|InstancedStaticMesh|SetCustomDataValue _instancedstaticmesh _index 0 (Math|Conversions|ToFloat(Integer) (Math|Float|Ceil (Math|Random|RandomFloatinRange -1.0 2.9999))) false)
      (Components|InstancedStaticMesh|SetCustomDataValue _instancedstaticmesh _index 1 (Math|Conversions|ToFloat(Integer) (Math|Float|Ceil (Math|Random|RandomFloatinRange -1.0 2.9999))) false))))